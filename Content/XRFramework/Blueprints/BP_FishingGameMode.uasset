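; Game mode for the XR fishing game that handles the result display between sets and the move to the results level.
; When a set completes, it spawns a result UI actor at a preset transform and passes it success and whether time is up.
; StartNextSetWithCleanup destroys that actor and starts the next set.
; Game end opens LV_GameResult, while the time-up event is empty.
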(event EventOnTimeUpBP)

(event EventOnEndGameBP
  (Game|OpenLevel(byObjectReference) "/Game/Maps/LV_GameResult.LV_GameResult"))

(event EventOnSetCompletedBP
  (params (bIsSuccess :type Boolean))
  (bind _returnvalue (Game|SpawnActorfromClass "/Game/UI/BP_SetResultUI.BP_SetResultUI_C" (Math|Transform|MakeTransform (Variables|Default|GetResultUILocation) (Variables|Default|GetResultUIRotation) "1.000000,1.000000,1.000000") "Undefined" "MultiplyWithRoot" 0 0))
  (Variables|Default|SetResultUIActor _returnvalue)
  (Default|SetResult _returnvalue bIsSuccess (Variables|Default|GetbIsTimeUp)))

(event EventBeginPlay)

(fn ConstructionScript)

(fn StartNextSetwithCleanup
  (Actor|DestroyActor (Variables|Default|GetResultUIActor))
  (Class|FishingGameModeBase|StartNextSet))