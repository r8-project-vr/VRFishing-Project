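; BP_Bird is an ambient bird actor that repeatedly flies straight across the sky above the player.
; Each pass picks a random horizontal direction and centers the path at a set height over the player pawn's current position.
; A timeline, rate-scaled by the flight duration, lerps the bird between the endpoints.
; On finish it hides the bird, waits briefly, then starts a new pass.
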(event Custom|StartFlight
  (Variables|Default|SetFlightDirection (Math|Vector|GetForwardVector (Math|Rotator|MakeRotator 0.0 0.0 (Math|Random|RandomFloatinRange 0.0 3.6e+02))))
  (Variables|Default|SetFlightCenter (+ (Transformation|GetActorLocation (Game|Player|GetPlayerPawn 0)) (Math|Vector|MakeVector 0.0 0.0 (Variables|Default|GetFlightHeight))))
  (bind _output_get (Variables|Default|SetStartLocation (- (Variables|Default|GetFlightCenter) (* (Variables|Default|GetFlightDirection) (Variables|Default|GetFlightDistance)))))
  (bind _output_get_2 (Variables|Default|SetEndLocation (+ (Variables|Default|GetFlightCenter) (* (Variables|Default|GetFlightDirection) (Variables|Default|GetFlightDistance)))))
  (Transformation|SetActorLocationAndRotation (Variables|Default|GetStartLocation) (Math|Rotator|FindLookatRotation _output_get _output_get_2))
  (Rendering|SetActorHiddenInGame false)
  (Components|Timeline|SetPlayRate (Variables|Default|GetTL_Flight) (/ 1.0 (Variables|Default|GetFlightDuration)))
  (bind _movealpha (Timeline|TL_Flight PlayFromStart)
    (:Update
      (Transformation|SetActorLocation (Math|Vector|Lerp(Vector) _output_get _output_get_2 _movealpha) false false))
    (:Finished
      (Rendering|SetActorHiddenInGame true)
      (Utilities|FlowControl|Delay 8.0)
      (CallFunction|StartFlight))))

(event EventBeginPlay
  (CallFunction|StartFlight))

(event Collision|EventActorBeginOverlap
  (params (OtherActor :type Actor%20Object%20Reference)))

(event EventTick
  (params (DeltaSeconds :type Float%20%28single-precision%29)))

(fn ConstructionScript)