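; BP_WindSpawner is an actor that periodically spawns wind visual effects around the player.
; On BeginPlay it calls SpawnWind, which spawns the NS_WindUndulation Niagara system at the player character's location when that character is valid.
; SpawnWind then re-arms itself on a timer with a random delay of a few seconds and prints an on-screen debug message.
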(event Custom|SpawnWind
  (bind _returnvalue (Game|GetPlayerCharacter 0))
  (Utilities|IsValid _returnvalue
    (:Is%20Valid
      (Niagara|SpawnSystematLocation "/Game/Effect/NS_WindUndulation.NS_WindUndulation" (+ (Transformation|GetActorLocation _returnvalue) (Math|Vector|MakeVector 0.0 0.0 0.0))))
    (:Is%20Not%20Valid
      _))
  (Utilities|Time|SetTimerbyEvent (delegate Custom|SpawnWind) (Math|Random|RandomFloatinRange 3.0 5.0))
  (Development|PrintString "風出てます" true true "(R=1.000000,G=0.933795,B=0.000000,A=1.000000)"))

(event EventBeginPlay
  (CallFunction|SpawnWind))

(event Collision|EventActorBeginOverlap
  (params (OtherActor :type Actor%20Object%20Reference)))

(event EventTick
  (params (DeltaSeconds :type Float%20%28single-precision%29)))

(fn ConstructionScript)