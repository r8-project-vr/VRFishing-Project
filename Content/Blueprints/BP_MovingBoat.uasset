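; BP_MovingBoat is a boat actor that travels in a straight line along the world Y axis and then removes itself.
; On BeginPlay it starts two audio components and sets its lifespan to TravelDistance divided by MoveSpeed, so it expires after covering that distance.
; Tick offsets its position by MoveSpeed scaled by delta time, without sweeping for collision.
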(event EventBeginPlay
  (Audio|Components|Audio|Play (Variables|Default|GetAudio) 0.0)
  (Audio|Components|Audio|Play (Variables|Default|GetAudio1) 0.0)
  (Actor|SetLifeSpan (/ (Variables|Default|GetTravelDistance) (Variables|Default|GetMoveSpeed))))

(event EventTick
  (params (DeltaSeconds :type Float%20%28single-precision%29))
  (Transformation|AddActorWorldOffset (Math|Vector|MakeVector 0.0 (* (Variables|Default|GetMoveSpeed) DeltaSeconds) 0.0)))

(fn ConstructionScript)